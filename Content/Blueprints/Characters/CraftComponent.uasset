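; Crafting component that matches items against gun or food recipes and turns them into a crafted item actor.
; Recipes come from the DataTable selected by RecipesDataType; lookups match item class and count, or find a recipe by its output.
; Craft notifies inputs, deducts recipe counts, then spawns and returns the result at a far-off location.
; Convert only finds a recipe and loops over its ingredients without acting; GetDataRows is empty.
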(fn Craft
  (params (Recipe :type ST%20Recipe%20Structure) (Items :type Array%20of%20Storage%20Item%20Object%20References))
  (bind (_item _items) (Utilities|Struct|BreakST_Recipe Recipe))
  (bind (_item_2 _count) (Utilities|Struct|BreakSTBeginItemInfo _item))
  (Utilities|FlowControl|Sequence
    (:then_0
      (for _array_element Items
        (Default|UsedtoCraft _array_element))
      (CallFunction|RemoveCraftedItems Items _items))
    (:then_1
      (Development|PrintString (Utilities|String|ToString(Integer) _count))
      (bind _returnvalue (Game|SpawnActorfromClass _item_2 (Math|Transform|MakeTransform "999999.000000,999999.000000,999999.000000") "AlwaysSpawn" 0 _count false))
      (Default|FreezePhysComponents _returnvalue false)
      (Rendering|SetActorHiddenInGame _returnvalue false)
      (Default|Crafted _returnvalue)
      (return _returnvalue))))

(fn RemoveCraftedItems
  (params (Items :type Array%20of%20Storage%20Item%20Object%20References) (Infos :type Array%20of%20ST%20Begin%20Item%20Info%20Structures))
  (LocalVariables|SetL_Items Items)
  (bind _array_element (Utilities|Array|ForEachLoopwithBreak Infos)
    (:LoopBody
      (bind (_array_element_2 _array_index) (Utilities|Array|ForEachLoopwithBreak (LocalVariables|GetL_Items) :!label _label)
        (:LoopBody
          (if (== (Utilities|GetClass _array_element_2) (.Item (Utilities|Struct|BreakSTBeginItemInfo _array_element)))
            (Default|SIRemoveItem _array_element_2 (.Count (Utilities|Struct|BreakSTBeginItemInfo _array_element)))
            (Utilities|Array|RemoveIndex (LocalVariables|GetL_Items) _array_index)
            (goto _label Break)))))))

(fn FindItemsbyRecipe
  (params (Recipe :type ST%20Recipe%20Structure) (InItems :type Array%20of%20Storage%20Item%20Object%20References))
  (LocalVariables|SetL_Recipe Recipe)
  (LocalVariables|SetL_InItems InItems)
  (bind _array_element (Utilities|Array|ForEachLoopwithBreak (.Items (Utilities|Struct|BreakST_Recipe (LocalVariables|GetL_Recipe))))
    (:LoopBody
      (bind _array_element_2 (Utilities|Array|ForEachLoopwithBreak (LocalVariables|GetL_InItems) :!label _label)
        (:LoopBody
          (if (== (Utilities|GetClass _array_element_2) (.Item (Utilities|Struct|BreakSTBeginItemInfo _array_element)))
            (bind _output_get (LocalVariables|SetL_TempItem _array_element_2))
            (Utilities|IsValid _output_get
              (:Is%20Valid
                (if (< (Variables|/Game/Blueprints/Storage/Items/StorageItem.StorageItem_C|GetCount _output_get) (.Count (Utilities|Struct|BreakSTBeginItemInfo _array_element)))
                  (LocalVariables|SetL_Found false)
                  (return false 0)
                  (else
                    (Utilities|Array|Add (LocalVariables|GetL_Items) (LocalVariables|GetL_TempItem))
                    (LocalVariables|SetL_Found true)
                    (goto _label Break)))))))
        (:Completed
          (if (not (LocalVariables|GetL_Found))
            (return false (Utilities|Array|MakeArray))))))
    (:Completed
      (return true (LocalVariables|GetL_Items)))))

(fn FindRecipebyItems
  (params (Items :type Array%20of%20Storage%20Item%20Object%20References))
  (LocalVariables|SetL_Items Items)
  (bind _rows (CallFunction|GetCraftDataRowNames))
  (bind _array_element (Utilities|Array|ForEachLoopwithBreak _rows :!label _label)
    (:LoopBody
      (bind _row (CallFunction|GetCraftDataRow _array_element))
      (bind _output_get (LocalVariables|SetL_Recipe _row))
      (LocalVariables|SetL_ItemsForRecipeWasNotFound false)
      (bind _array_element_2 (Utilities|Array|ForEachLoopwithBreak (.Items (Utilities|Struct|BreakST_Recipe _output_get)) :!label _label_2)
        (:LoopBody
          (LocalVariables|SetL_RecipeWasFound false)
          (bind _array_element_3 (Utilities|Array|ForEachLoopwithBreak (LocalVariables|GetL_Items) :!label _label_3)
            (:LoopBody
              (if (== (Utilities|GetClass _array_element_3) (.Item (Utilities|Struct|BreakSTBeginItemInfo _array_element_2)))
                (if (>= (Variables|/Game/Blueprints/Storage/Items/StorageItem.StorageItem_C|GetCount _array_element_3) (.Count (Utilities|Struct|BreakSTBeginItemInfo _array_element_2)))
                  (LocalVariables|SetL_RecipeWasFound true)
                  (goto _label_3 Break))))
            (:Completed
              (if (not (LocalVariables|GetL_RecipeWasFound))
                (LocalVariables|SetL_ItemsForRecipeWasNotFound true)
                (goto _label_2 Break)))))
        (:Completed
          (if (not (LocalVariables|GetL_ItemsForRecipeWasNotFound))
            (LocalVariables|SetL_RecipeWasFound true)
            (goto _label Break)))))
    (:Completed
      (return (LocalVariables|GetL_RecipeWasFound) (LocalVariables|GetL_Recipe)))))

(fn FindConvertRecipebyItem
  (params (Item :type Storage%20Item%20Object%20Reference))
  (LocalVariables|SetL_Item Item)
  (bind _rows (CallFunction|GetCraftDataRowNames))
  (for _array_element _rows
    (bind _row (CallFunction|GetCraftDataRow _array_element))
    (if (== (.Item (Utilities|Struct|BreakSTBeginItemInfo (.Item (Utilities|Struct|BreakST_Recipe _row)))) (Utilities|GetClass (LocalVariables|GetL_Item)))
      (return true _row)))
  (return false ""))

(fn Convert
  (params (Item :type Storage%20Item%20Object%20Reference))
  (bind (_recipefound _recipe) (CallFunction|FindConvertRecipebyItem Item))
  (bind _output_get (LocalVariables|SetL_Recipe _recipe))
  (if _recipefound
    (for _array_element (.Items (Utilities|Struct|BreakST_Recipe _output_get))
      _)))

(fn GetDataRows)

(fn GetCraftDataRow
  (params (RowName :type Name))
  (LocalVariables|SetL_RowName RowName)
  (Utilities|FlowControl|Sequence
    (:then_0
      (switch Utilities|FlowControl|Switch|SwitchonE_RecipeDataType (Variables|Default|GetRecipesDataType)
        (:NewEnumerator1
          (bind _returnvalue (Utilities|GetDataTableRow "/Game/Blueprints/Recipes/DT_GunRecipes.DT_GunRecipes" (LocalVariables|GetL_RowName))
            (:then
              (LocalVariables|SetL_Row _returnvalue))))
        (:NewEnumerator0
          (bind _returnvalue_2 (Utilities|GetDataTableRow "/Game/Blueprints/Recipes/Dt_FoodRecipes.Dt_FoodRecipes" (LocalVariables|GetL_RowName))
            (:then
              (LocalVariables|SetL_Row _returnvalue_2))))))
    (:then_1
      (return (LocalVariables|GetL_Row)))))

(fn GetCraftDataRowNames
  (Utilities|FlowControl|Sequence
    (:then_0
      (switch Utilities|FlowControl|Switch|SwitchonE_RecipeDataType (Variables|Default|GetRecipesDataType)
        (:NewEnumerator1
          (bind _outrownames (DataTable|GetDataTableRowNames "/Game/Blueprints/Recipes/DT_GunRecipes.DT_GunRecipes"))
          (LocalVariables|SetL_Rows _outrownames))
        (:NewEnumerator0
          (bind _outrownames_2 (DataTable|GetDataTableRowNames "/Game/Blueprints/Recipes/Dt_FoodRecipes.Dt_FoodRecipes"))
          (LocalVariables|SetL_Rows _outrownames_2))))
    (:then_1
      (return (LocalVariables|GetL_Rows)))))