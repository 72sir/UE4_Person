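; Player controller for the survival character that owns the HUD, inventory and item exchange UI.
; On BeginPlay it builds the HUD, hands the controlled SurvivalCharacter to its sub-widgets and pre-creates the inventory.
; Tab toggles the inventory, while Escape or Backspace closes the exchange widget opened through ExchangeWidget with an exchange component.
; Both panels share UIControl, which switches cursor visibility, input mode and pawn input.
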(event EventBeginPlay
  (Utilities|FlowControl|Sequence
    (:then_0
      (CallFunction|WHUD-Stats)
      (UserInterface|CreateWidget "/Game/UI/MainHUD/W_HUD-RPGStats.W_HUD-RPGStats_C" self)
      (Variables|/Game/UI/MainHUD/W_HUD-RPGStats.W_HUD-RPGStats_C|SetCharacter (Variables|/Game/UI/MainHUD/W_HUD.W_HUD_C|GetW_HUD-RPGStats_29 (Variables|Default|GetW_HUD)) (.AsSurvival%20Character (Utilities|Casting|CastToSurvivalCharacter (Pawn|GetControlledPawn)))))
    (:then_1
      (bind _returnvalue (UserInterface|CreateWidget "/Game/UI/Inventory/W_Inventory.W_Inventory_C" self))
      (Variables|Default|SetW_Inventory _returnvalue))))

(event Input|KeyboardEvents|Tab
  (params (Key :type Key%20Structure :default "AnyKey"))
  (:Pressed
    (CallFunction|ToggleInventory)))

(event Input|KeyboardEvents|Backspace
  (params (Key :type Key%20Structure :default "AnyKey"))
  (:Pressed
    (Utilities|IsValid (Variables|Default|GetW_ExchangeWidget)
      (:Is%20Valid
        (CallFunction|ExchangeWidget 0 true)))))

(event Input|KeyboardEvents|Escape
  (params (Key :type Key%20Structure :default "AnyKey"))
  (:Pressed
    (Utilities|IsValid (Variables|Default|GetW_ExchangeWidget)
      (:Is%20Valid
        (CallFunction|ExchangeWidget 0 true)))))

(fn ConstructionScript)

(fn WHUD-Stats
  (bind _returnvalue (UserInterface|CreateWidget "/Game/UI/MainHUD/W_HUD.W_HUD_C" self))
  (bind _output_get (Variables|Default|SetW_HUD _returnvalue))
  (UserInterface|Viewport|AddtoViewport _output_get 0)
  (bind _output_get_2 (Variables|/Game/UI/MainHUD/W_HUD-HealtStats.W_HUD-HealtStats_C|SetCharacter (Variables|/Game/UI/MainHUD/W_HUD.W_HUD_C|GetW_HUD-HealtStats_76 (Variables|Default|GetW_HUD)) (.AsSurvival%20Character (Utilities|Casting|CastToSurvivalCharacter (Pawn|GetControlledPawn)))))
  (Variables|/Game/UI/MainHUD/W_HUD-Items.W_HUD-Items_C|SetCharacter (Variables|/Game/UI/MainHUD/W_HUD.W_HUD_C|GetW_HUD-Items_59 (Variables|Default|GetW_HUD)) _output_get_2))

(fn ToggleInventory
  (if (not (Variables|Default|GetInventoryShow))
    ;[1 1 1] Block inventory, block character input
    (UserInterface|Viewport|AddtoViewport (Variables|Default|GetW_Inventory) 0)
    (Default|InventoryAddedtoViewport (Variables|Default|GetW_Inventory))
    (Variables|Default|SetInventoryShow true)
    (CallFunction|UIControl true)
    (else
      ;[1 1 1] Hide inputs return inputs
      (Widget|RemovefromParent (Variables|Default|GetW_Inventory))
      (Variables|Default|SetInventoryShow false)
      (CallFunction|UIControl false))))

(fn ExchangeWidget
  (params (ExchangeComponent :type Storage%20Component%20Object%20Reference) (Remove :type Boolean))
  (if Remove
    (Widget|RemovefromParent (Variables|Default|GetW_ExchangeWidget))
    (Variables|Default|SetW_ExchangeWidget 0)
    (CallFunction|UIControl false)
    (else
      (bind _returnvalue (UserInterface|CreateWidget "/Game/UI/Inventory/W_ItemExchange.W_ItemExchange_C" self ExchangeComponent))
      (bind _output_get (Variables|Default|SetW_ExchangeWidget _returnvalue))
      (UserInterface|Viewport|AddtoViewport _output_get 0)
      (CallFunction|UIControl true))))

(fn UIControl
  (params (Activate :type Boolean))
  (if Activate
    (Variables|Default|SetbShowMouseCursor true)
    (Input|SetInputModeGameandUI self (Variables|Default|GetW_Inventory) "DoNotLock" true)
    (Input|DisableInput (Pawn|GetControlledPawn) self)
    (else
      (Variables|Default|SetbShowMouseCursor false)
      (Input|EnableInput (Pawn|GetControlledPawn) self)
      (Input|SetInputModeGameOnly self))))