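; Equipment component that tracks the items equipped in a character's head, torso, legs, feet and weapon slots.
; EquipItem empties the target slot through UnEquipItem, which notifies the old item and clears the reference, then stores the new one.
; Armor slots only hold references, while weapons are cast and snapped to the Skt_Weapon socket on SurvivalCharacter's first-person or body mesh, depending on the active camera.
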(event EventBeginPlay)

(event EventTick
  (params (DeltaSeconds :type Float%20%28single-precision%29)))

(fn EquipItem
  (params (Item :type Equip%20Able%20Item%20Object%20Reference) (Part :type E_EquipPart%20Enum))
  (LocalVariables|SetL_Item Item)
  (CallFunction|UnEquipItem Part)
  (switch Utilities|FlowControl|Switch|SwitchonE_EquipPart Part
    (:NewEnumerator0
      (Variables|Default|SetHead (LocalVariables|GetL_Item)))
    (:NewEnumerator1
      (Variables|Default|SetTorso (LocalVariables|GetL_Item)))
    (:NewEnumerator2
      (Variables|Default|SetLegs (LocalVariables|GetL_Item)))
    (:NewEnumerator3
      (Variables|Default|SetFoots (LocalVariables|GetL_Item)))
    (:NewEnumerator4
      (CallFunction|EquipWeapon (LocalVariables|GetL_Item))))
  (return true))

(fn UnEquipItem
  (params (Part :type E_EquipPart%20Enum))
  (bind (_equipped _item) (CallFunction|PartEquipped Part))
  (if _equipped
    (Default|UnEquipItem _item)
    (switch Utilities|FlowControl|Switch|SwitchonE_EquipPart Part
      (:NewEnumerator0
        (Variables|Default|SetHead 0))
      (:NewEnumerator1
        (Variables|Default|SetTorso 0))
      (:NewEnumerator2
        (Variables|Default|SetLegs 0))
      (:NewEnumerator3
        (Variables|Default|SetFoots 0))
      (:NewEnumerator4
        (Variables|Default|SetWeapon 0)))
    (return true)
    (else
      (return false))))

(fn PartEquipped
  (params (Part :type E_EquipPart%20Enum))
  (bind _weapon (Variables|Default|GetWeapon))
  (bind _foots (Variables|Default|GetFoots))
  (bind _torso (Variables|Default|GetTorso))
  (bind _legs (Variables|Default|GetLegs))
  (bind _head (Variables|Default|GetHead))
  (bind _returnvalue (Utilities|Select :Index Part :NewEnumerator0 _head :NewEnumerator1 _torso :NewEnumerator2 _legs :NewEnumerator3 _foots :NewEnumerator4 _weapon))
  (return (Utilities|IsValid _returnvalue) _returnvalue))

(fn EquipWeapon
  (params (Item :type Equip%20Able%20Item%20Object%20Reference))
  (bind _asweapon (Utilities|Casting|CastToWeapon Item)
    (:then
      (Variables|Default|SetWeapon _asweapon)
      (CallFunction|AttachWeapon true))
    (:CastFailed
      (Development|PrintString "default cast to weapon"))))

(fn AttachWeapon
  (params (Attach :type Boolean))
  (if Attach
    (bind _assurvival_character (Utilities|Casting|CastToSurvivalCharacter (Components|GetOwner)))
    (Transformation|AttachComponentToComponent (Variables|Default|GetWeapon) (select (Variables|/Game/Blueprints/Characters/SurvivalCharacter.SurvivalCharacter_C|GetFirstCameraActive _assurvival_character) (Variables|/Game/Blueprints/Characters/SurvivalCharacter.SurvivalCharacter_C|GetFirstPersonMesh _assurvival_character) (Variables|/Script/Engine.Character|GetMesh _assurvival_character)) "Skt_Weapon" "SnapToTarget" "SnapToTarget" "SnapToTarget" true)
    (else
      (Transformation|DetachFromActor (Variables|Default|GetWeapon) "KeepWorld" "KeepWorld" "KeepWorld"))))