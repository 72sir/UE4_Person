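; Health and stamina stats Blueprint for characters, with on-screen debug printing of both values.
; ChangeHealth adds a signed value capped at 100 and calls HeathEnd once, guarded by a flag, when health reaches zero or below.
; UseStamina moves stamina at constant speed toward empty while in use or full otherwise, scaled by world delta time.
; Tick is empty, so these functions rely on external callers.
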(event EventTick
  (params (DeltaSeconds :type Float%20%28single-precision%29)))

(fn ChangeHealth
  (params (Value :type Float%20%28single-precision%29))
  (if (<= (Variables|healt|GetHealth) 1e+02)
    (bind _output_get (Variables|healt|SetHealth (Math|Float|Min(Float) (+ Value (Variables|healt|GetHealth)) 1e+02)))
    (if (and (<= _output_get 0.0) (not (Variables|Healt|GetNoHealt)))
      (Variables|Healt|SetNoHealt true)
      (Default|CallHeathEnd))))

(fn DisplayStats
  (Development|PrintString (Utilities|String|Append "Health: " (Utilities|String|ToString(Float) (Variables|healt|GetHealth))) true true "(R=0.000000,G=0.660000,B=1.000000,A=1.000000)" 0.0)
  (Development|PrintString (Utilities|String|Append " Stamina: " (Utilities|String|ToString(Float) (Variables|Stamina|GetfStamina))) true true "(R=1.000000,G=0.000000,B=0.193894,A=1.000000)" 0.0))

(fn UseStamina
  (params (Use :type Boolean))
  (Variables|Stamina|SetfStamina (Math|Interpolation|FInterptoConstant (Variables|Stamina|GetfStamina) (Math|Float|SelectFloat 0.0 1e+02 Use) (Utilities|Time|GetWorldDeltaSeconds) (Variables|Stamina|GetfStaminaSpeed))))