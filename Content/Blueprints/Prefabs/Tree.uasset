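; Choppable tree prefab that yields berries when damaged and wood once felled.
; Any damage spawns berries at a random offset from a component, but only axe hits update Condition, computed as Damage minus Condition rather than the reverse.
; At zero or below, it fires TreeFalls, whose bound timeline pitches the actor toward 90 degrees.
; Interacting with the fallen tree adds its construction-randomized wood count to the character's storage and destroys it.
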(event Custom|PlayFallAnim
  (params (Tree :type Actor%20Object%20Reference) (instigator :type Pawn%20Object%20Reference))
  (bind _returnvalue (Transformation|GetActorRotation))
  ;[1 1 1] Anim
  (bind _newtrack_0 (Timeline|Timeline_0 PlayFromStart)
    (:Update
      (Transformation|SetActorRotation (Math|Rotator|MakeRotator (.roll _returnvalue) (Math|Float|Lerp (.pitch _returnvalue) 9e+01 _newtrack_0) (.yaw _returnvalue))))))

(event EventBeginPlay
  (EventDispatchers|BindEventtoTreeFalls (delegate Custom|PlayFallAnim)))

(event Game|Damage|EventAnyDamage
  (params (Damage :type Float%20%28single-precision%29) (DamageType :type Damage%20Type%20Object%20Reference) (InstigatedBy :type Controller%20Object%20Reference) (DamageCauser :type Actor%20Object%20Reference))
  ;[1 1 1] TreeHit
  (CallFunction|HitATree Damage InstigatedBy DamageCauser)
  ;[1 1 1] Ягоды при ударе по дереву
  (Game|SpawnActorfromClass "/Game/Blueprints/Storage/Items/EquipAbles/Food/Food_Berries.Food_Berries_C" (Math|Transform|MakeTransform (+ (Transformation|GetWorldLocation (Variables|Default|Get2)) (* (Math|Random|RandomUnitVector) (Math|Random|RandomFloatinRange 0.0 (Variables|/Script/Engine.SphereComponent|GetSphereRadius (Variables|Default|Get2))))) "0, 0, 0" "1,1,1") "AlwaysSpawn" 0 1 true))

(fn ConstructionScript
  (Variables|Default|SetWoodCount (Math|Random|RandomIntegerinRange 5 10)))

(fn HitATree
  (params (Damage :type Float%20%28single-precision%29) (Instigator :type Controller%20Object%20Reference) (Causer :type Object%20Object%20Reference))
  (if (== (Utilities|GetClass Causer) "/Game/Blueprints/Storage/Items/EquipAbles/Weapons/Weapon_Axe.Weapon_Axe_C")
    (bind _output_get (Variables|Default|SetCondition (- Damage (Variables|Default|GetCondition))))
    (if (<= _output_get 0.0)
      (Variables|Default|SetFallen true)
      (Default|CallTreeFalls self (Pawn|GetControlledPawn Instigator))
      (return true true)
      (else
        (return false true)))
    (else
      (return false false))))

(fn Interact
  (params (Character :type Survival%20Character%20Object%20Reference))
  (if (Variables|Default|GetFallen)
    (Default|CreateItems (Variables|/Game/Blueprints/Characters/SurvivalCharacter.SurvivalCharacter_C|GetStorageComponent Character) (Utilities|Array|MakeArray (Utilities|Struct|MakeSTBeginItemInfo "/Game/Blueprints/Storage/Items/Item_Wood.Item_Wood_C" (Variables|Default|GetWoodCount))))
    (Actor|DestroyActor)
    (return true "")
    (else
      (return false "Tree is not fallen"))))