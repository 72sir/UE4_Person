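; Inventory storage component that holds item actors in a paged X/Y grid under a total weight limit, spawning its starting items at BeginPlay.
; Adding requires weight room and a first-fit free slot, then merges stackable items into the first same-class item or places them as new entries.
; Slot occupancy comes from querying each stored item.
; Removal handles partial stacks and feeds transfers between storages and drops in front of the owner.
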(event EventBeginPlay
  (CallFunction|CreateItems (Variables|Default|GetBeginItems)))

(fn SCAddItem
  (params (Item :type Storage%20Item%20Object%20Reference))
  (bind _output_get (LocalVariables|SetL_Item Item))
  (bind (_canadd _x _y _page) (CallFunction|CheckifItemCanbeAdded _output_get))
  (LocalVariables|SetL_X _x)
  (LocalVariables|SetL_Y _y)
  (LocalVariables|SetL_Page _page)
  (if _canadd
    (if (.CanBeStack (CallFunction|ChackItemsforStack (LocalVariables|GetL_Item)))
      ;[1 1 1] StackItem
      (Variables|/Game/Blueprints/Storage/Items/StorageItem.StorageItem_C|SetCount (.StackIn (CallFunction|ChackItemsforStack (LocalVariables|GetL_Item))) (+ (Variables|/Game/Blueprints/Storage/Items/StorageItem.StorageItem_C|GetCount (LocalVariables|GetL_Item)) (Variables|/Game/Blueprints/Storage/Items/StorageItem.StorageItem_C|GetCount (.StackIn (CallFunction|ChackItemsforStack (LocalVariables|GetL_Item))))))
      (CallFunction|ChangeTotalWeight (Default|GetItemWeight (LocalVariables|GetL_Item) true))
      (Default|DestroyItem (LocalVariables|GetL_Item))
      (return true)
      (else
        ;[1 1 1] AddNewItem
        (Utilities|Array|Add (Variables|Default|GetItems) (LocalVariables|GetL_Item))
        (CallFunction|ChangeTotalWeight (Default|GetItemWeight (LocalVariables|GetL_Item) true (Variables|/Game/Blueprints/Storage/Items/StorageItem.StorageItem_C|GetCount (LocalVariables|GetL_Item))))
        (Default|ItemAddedtoStorage (LocalVariables|GetL_Item) self (LocalVariables|GetL_X) (LocalVariables|GetL_Y) (LocalVariables|GetL_Page))
        (return true)))
    (else
      (return false))))

(fn SCRemoveItem
  (params (StorageItem :type Storage%20Item%20Object%20Reference) (Count :type Integer) (RemoveAll :type Boolean) (Destroy :type Boolean))
  (Utilities|IsValid StorageItem
    (:Is%20Valid
      (bind _output_get (LocalVariables|SetL_Item StorageItem))
      (LocalVariables|SetL_Count (Math|Integer|SelectInt (Variables|/Game/Blueprints/Storage/Items/StorageItem.StorageItem_C|GetCount _output_get) Count RemoveAll))
      (if (== (.Storage (Default|IsinStorage (LocalVariables|GetL_Item))) self)
        (bind _removedall (CallFunction|RemoveStackedItem (LocalVariables|GetL_Item) (LocalVariables|GetL_Count)))
        (CallFunction|ChangeTotalWeight (* (Default|GetItemWeight (LocalVariables|GetL_Item) _removedall (LocalVariables|GetL_Count)) -1.0))
        (if _removedall
          (Utilities|Array|RemoveItem (Variables|Default|GetItems) (LocalVariables|GetL_Item))
          (Default|ItemRemovedfromStorage (LocalVariables|GetL_Item) self)
          (if Destroy
            (Default|DestroyItem (LocalVariables|GetL_Item))
            (return true)
            (else
              (return true)))
          (else
            (return (> (LocalVariables|GetL_Count) 0))))
        (else
          (return false))))
    (:Is%20Not%20Valid
      (Development|PrintString "ЧТО ТО ПУСТО ПОТОМУ ЧТО ЧЕГО ТО НЕТ"))))

(fn CheckifItemCanbeAdded
  (params (Item :type Storage%20Item%20Object%20Reference))
  (bind _output_get (LocalVariables|SetL_Item Item))
  (if (> (+ (Variables|Default|GetStorageTotalWeight) (Default|GetItemWeight _output_get true)) (Variables|Default|GetStorageMaxWeight))
    _
    (else
      (bind (_nofreeeslot _x _y _page) (CallFunction|CheckFreeSlotforItem (LocalVariables|GetL_Item)))
      (if _nofreeeslot
        _
        (else
          (return true _x _y _page)))))
  (return false 0 0 0))

(fn ChangeTotalWeight
  (params (Value :type Float%20%28single-precision%29))
  (Variables|Default|SetStorageTotalWeight (+ Value (Variables|Default|GetStorageTotalWeight))))

(fn DropItemtoWorld
  (params (Item :type Storage%20Item%20Object%20Reference) (Count :type Integer) (DropAll :type Boolean))
  (LocalVariables|SetL_Item Item)
  (if DropAll
    ;[1 1 1] DropSome
    (bind _removed (CallFunction|SCRemoveItem (LocalVariables|GetL_Item) (LocalVariables|GetL_Count) DropAll false :!label _label))
    (if _removed
      (bind _returnvalue (Game|SpawnActorfromClass (Utilities|GetClass (LocalVariables|GetL_Item)) (Math|Transform|MakeTransform "0, 0, 0" "0.000000, 0, 0" (Transformation|GetWorldScale (Variables|/Game/Blueprints/Storage/Items/StorageItem.StorageItem_C|GetDefaultSceneRoot (LocalVariables|GetL_Item)))) "AlwaysSpawn" 0 (LocalVariables|GetL_Count) (Variables|/Game/Blueprints/Storage/Items/StorageItem.StorageItem_C|GetCanBeStacked (LocalVariables|GetL_Item))))
      (Default|FreezePhysComponents _returnvalue true)
      (Default|DroppedtoWorld _returnvalue (CallFunction|DropLocation)))
    (else
      (bind _output_get (LocalVariables|SetL_Count Count))
      (if (.FullStack (CallFunction|IsFullStackbyCount (LocalVariables|GetL_Item) _output_get))
        ;[1 1 1] DropAll
        (bind _removed_2 (CallFunction|SCRemoveItem (LocalVariables|GetL_Item) (LocalVariables|GetL_Count) false false))
        (if _removed_2
          (Default|DroppedtoWorld (LocalVariables|GetL_Item) (CallFunction|DropLocation)))
        (else
          (goto _label))))))

(fn GetItems
  (return (Variables|Default|GetItems)))

(fn PlacetoAnotherStorage
  (params (Item :type Storage%20Item%20Object%20Reference) (Storage :type Storage%20Component%20Object%20Reference))
  (bind _output_get (LocalVariables|SetL_Item_1 Item))
  (bind _output_get_2 (LocalVariables|SetL_Storage Storage))
  (bind _canadd (CallFunction|CheckifItemCanbeAdded _output_get_2 _output_get))
  (if _canadd
    (bind _removed (CallFunction|SCRemoveItem (LocalVariables|GetL_Item_1) (Variables|/Game/Blueprints/Storage/Items/StorageItem.StorageItem_C|GetCount (LocalVariables|GetL_Item_1)) false false))
    (if _removed
      (bind _added (CallFunction|SCAddItem (LocalVariables|GetL_Storage) (LocalVariables|GetL_Item_1)))
      (return _added)
      (else
        (return false)))
    (else
      (return false))))

(fn CreateItems
  (params (Items :type Array%20of%20ST%20Begin%20Item%20Info%20Structures))
  (bind _array_element (Utilities|Array|ForEachLoopwithBreak Items :!label _label)
    (:LoopBody
      (if (CallFunction|CheckifItemCanbeCreated (.Item (Utilities|Struct|BreakSTBeginItemInfo _array_element)) (.Count (Utilities|Struct|BreakSTBeginItemInfo _array_element)))
        (bind _returnvalue (Game|SpawnActorfromClass (.Item (Utilities|Struct|BreakSTBeginItemInfo _array_element)) (Math|Transform|MakeTransform "0, 0, 0") "AlwaysSpawn" 0 (.Count (Utilities|Struct|BreakSTBeginItemInfo _array_element)) true))
        (Utilities|Array|Add (LocalVariables|GetL_CreatedItems) 0)
        (CallFunction|SCAddItem _returnvalue)
        (else
          (goto _label Break))))
    (:Completed
      (return (LocalVariables|GetL_CreatedItems)))))

(fn CheckifItemCanbeCreated
  (params (Item :type Storage%20Item%20Class%20Reference) (Count :type Integer))
  (if (> (+ (Variables|Default|GetStorageTotalWeight) (* Count (.Weight (Utilities|GetClassDefaults Item)))) (Variables|Default|GetStorageMaxWeight))
    (return false)
    (else
      (return true))))

(fn ChackItemsforStack
  (params (Item :type Storage%20Item%20Object%20Reference))
  (bind _returnvalue (Utilities|GetClass Item))
  (bind (_wasfound _item) (CallFunction|GetIteminStoragebyClass _returnvalue))
  (if (Variables|/Game/Blueprints/Storage/Items/StorageItem.StorageItem_C|GetCanBeStacked Item)
    (return _wasfound _item)
    (else
      (return false 0))))

(fn RemoveStackedItem
  (params (Item%20 :type Storage%20Item%20Object%20Reference) (Count :type Integer))
  (bind _output_get (LocalVariables|SetL_Item Item%20))
  (bind _output_get_2 (LocalVariables|SetbCount (.FullStack (CallFunction|IsFullStackbyCount _output_get Count))))
  (if _output_get_2
    _
    (else
      (Variables|/Game/Blueprints/Storage/Items/StorageItem.StorageItem_C|SetCount (LocalVariables|GetL_Item) (.Remain (CallFunction|IsFullStackbyCount _output_get Count)))
      (Default|CallSIItemRemoved (LocalVariables|GetL_Item) (LocalVariables|GetL_Item) Count)))
  (return (LocalVariables|GetbCount)))

(fn IsFullStackbyCount
  (params (Item :type Storage%20Item%20Object%20Reference) (Count :type Integer))
  (bind _returnvalue (- (Variables|/Game/Blueprints/Storage/Items/StorageItem.StorageItem_C|GetCount Item) Count))
  (Utilities|IsValid Item
    (:Is%20Valid
      (return (<= _returnvalue 0) _returnvalue))
    (:Is%20Not%20Valid
      (return false 0))))

(fn DropLocation
  (bind _returnvalue (Components|GetOwner))
  (return (+ (Transformation|GetActorLocation _returnvalue) (* (Transformation|GetActorForwardVector _returnvalue) (Variables|Default|GetDropDistance)))))

(fn GetIteminStoragebyClass
  (params (Class :type Storage%20Item%20Class%20Reference))
  (bind _array_element (Utilities|Array|ForEachLoopwithBreak (Variables|Default|GetItems) :!label _label)
    (:LoopBody
      (if (== (Utilities|GetClass _array_element) Class)
        (LocalVariables|SetL_Item _array_element)
        (LocalVariables|SetL_ItemFound true)
        (goto _label Break)))
    (:Completed
      (return (LocalVariables|GetL_ItemFound) (LocalVariables|GetL_Item)))))

(fn CheckSlot
  (params (Page :type Integer) (X :type Integer) (Y :type Integer) (CheckExactSlot :type Boolean))
  (LocalVariables|SetL_Page Page)
  (LocalVariables|SetL_X X)
  (LocalVariables|SetL_Y Y)
  (Utilities|FlowControl|Sequence
    (:then_0
      ;[1 1 1] Check for slot inventory borders
      (Utilities|FlowControl|Sequence
        (:then_0
          (if (or (> (LocalVariables|GetL_Page) (Variables|Default|GetStorageSizePages)) (< (LocalVariables|GetL_Page) 1))
            (return 0 false)))
        (:then_1
          (if (or (>= (LocalVariables|GetL_X) (Variables|Default|GetStorageSizeX)) (< (LocalVariables|GetL_X) 0))
            (return 0 false)))
        (:then_2
          (if (or (>= (LocalVariables|GetL_Y) (Variables|Default|GetStorageSizeY)) (< (LocalVariables|GetL_Y) 0))
            (return 0 false)))))
    (:then_1
      (bind _array_element (Utilities|Array|ForEachLoopwithBreak (Variables|Default|GetItems) :!label _label)
        (:LoopBody
          (if (select CheckExactSlot (|Checkexactlocation _array_element) (Default|CheckItItemIsinSlot _array_element (LocalVariables|GetL_X) (LocalVariables|GetL_Y) (LocalVariables|GetL_Page)))
            (LocalVariables|SetL_Item _array_element)
            (goto _label Break)))))
    (:then_2
      (return (LocalVariables|GetL_Item) (not (Utilities|IsValid (LocalVariables|GetL_Item)))))))

(fn CheckFreeSlotforItem
  (params (Item :type Storage%20Item%20Object%20Reference))
  (LocalVariables|SetL_Item Item)
  (bind _index (Utilities|FlowControl|ForLoopwithBreak 1 (Variables|Default|GetStorageSizePages))
    (:LoopBody
      (LocalVariables|SetL_Page _index)
      (bind _index_2 (Utilities|FlowControl|ForLoopwithBreak 0 (- (Variables|Default|GetStorageSizeY) 1))
        (:LoopBody
          (LocalVariables|SetL_Y _index_2)
          (bind _index_3 (Utilities|FlowControl|ForLoopwithBreak 0 (- (Variables|Default|GetStorageSizeX) 1))
            (:LoopBody
              (LocalVariables|SetL_X _index_3)
              (if (.Free (CallFunction|CheckSlot (LocalVariables|GetL_Page) (LocalVariables|GetL_X) (LocalVariables|GetL_Y) false))
                (bind _slotsarefree (CallFunction|CheckSlotsforItem (LocalVariables|GetL_Item) (LocalVariables|GetL_X) (LocalVariables|GetL_Y) (LocalVariables|GetL_Page)))
                (if _slotsarefree
                  (return false (LocalVariables|GetL_X) (LocalVariables|GetL_Y) (LocalVariables|GetL_Page)))))))))
    (:Completed
      (return true 0 0 0))))

(fn CheckSlotsforItem
  (params (Item :type Storage%20Item%20Object%20Reference) (X :type Integer) (Y :type Integer) (Page :type Integer))
  (LocalVariables|SetL_Item Item)
  (LocalVariables|SetL_X X)
  (LocalVariables|SetL_Y Y)
  (LocalVariables|SetL_Page Page)
  (bind _index (Utilities|FlowControl|ForLoopwithBreak 0 (- (.SizeY (Default|LocateItem (LocalVariables|GetL_Item))) 1))
    (:LoopBody
      (LocalVariables|SetL_Size_Y _index)
      (bind _index_2 (Utilities|FlowControl|ForLoopwithBreak 0 (- (.SizeX (Default|LocateItem (LocalVariables|GetL_Item))) 1))
        (:LoopBody
          (LocalVariables|SetL_Size_X _index_2)
          (if (or (!= (LocalVariables|GetL_Size_X) 0) (!= (LocalVariables|GetL_Size_Y) 0))
            (if (not (.Free (CallFunction|CheckSlot (LocalVariables|GetL_Page) (+ (LocalVariables|GetL_Size_X) (LocalVariables|GetL_X)) (+ (LocalVariables|GetL_Size_Y) (LocalVariables|GetL_Y)) false)))
              (return false))))))
    (:Completed
      (return true))))

(fn ChangeItemLocation
  (params (Item :type Storage%20Item%20Object%20Reference) (X :type Integer) (Y :type Integer) (Page :type Integer))
  (bind _slotsarefree (CallFunction|CheckSlotsforItem Item X Y Page))
  (if _slotsarefree
    (Default|RelocateItem Item X Y Page)
    (return true)
    (else
      (return false))))